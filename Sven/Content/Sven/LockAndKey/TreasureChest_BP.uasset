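; Treasure chest Blueprint for a lock-and-key interaction, opened when the player holds a key.
; It caches the first-person character on BeginPlay, and Interact checks that character's HasKey2, printing "Locked" without it.
; With the key, a FlipFlop plays a timeline on every other call to drive the lid's roll.
; The Lerp endpoints are both zero, so the lid stays at zero rotation, and no closing branch exists.
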(event EventBeginPlay
  (bind _asfirst_person_character (Utilities|Casting|CastToFirstPersonCharacter (Game|GetPlayerCharacter 0)))
  (Variables|Default|SetPlayer%20Character _asfirst_person_character))

(event EventInteract
  (params (Interacter :type Actor%20Object%20Reference))
  (Variables|Default|SetIsUnlocked true)
  (if true
    (if (Variables|/Game/FirstPersonBP/Blueprints/FirstPersonCharacter.FirstPersonCharacter_C|GetHasKey2? (Variables|Default|GetPlayer%20Character))
      (Utilities|FlowControl|FlipFlop :!label _label
        (:A
          (bind _newtrack_0 (Timeline|Timeline_0 Play)
            (:Update
              (Transformation|SetRelativeRotation (Variables|Default|Getchest_final_chest_top) (Math|Rotator|MakeRotator (Math|Float|Lerp 0.0 0.0 _newtrack_0) 0.0 0.0) false false)))))
      (else
        (Development|PrintString "Locked")))
    (else
      (goto _label))))

(fn ConstructionScript)