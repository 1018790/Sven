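; Key1_Pickup_BP is a key pickup for a lock-and-key system that also updates the player's objective.
; On BeginPlay it casts player character 0 to FirstPersonCharacter and caches the reference.
; Its Interact event sets HasKey1 on that character, writes the objective title and description from its own variables, then destroys the pickup.
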(event EventBeginPlay
  ;[1 1 1] Casting to First Person
  (bind _asfirst_person_character (Utilities|Casting|CastToFirstPersonCharacter (Game|GetPlayerCharacter 0)))
  (Variables|Default|SetPlayer%20Character _asfirst_person_character))

(event EventInteract
  (params (Interacter :type Actor%20Object%20Reference))
  (bind _player_character (Variables|Default|GetPlayer%20Character))
  ;[1 1 1] If Key is picked up, Change Objective
  (Variables|/Game/FirstPersonBP/Blueprints/FirstPersonCharacter.FirstPersonCharacter_C|SetHasKey1? _player_character true)
  (Variables|/Game/FirstPersonBP/Blueprints/FirstPersonCharacter.FirstPersonCharacter_C|SetPlayerObj _player_character (Variables|Default|GetPlayer%20Objective%20Title))
  (Variables|/Game/FirstPersonBP/Blueprints/FirstPersonCharacter.FirstPersonCharacter_C|SetPlayerObjDesc _player_character (Variables|Default|GetPlayer%20Objective%20Description))
  (Actor|DestroyActor))

(fn ConstructionScript)