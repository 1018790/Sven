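; Interactable bedroom door that either swings open and closed or shows the player why it stays shut.
; On Interact, flags pick the case: the parents' bedroom door opens freely or checks the first-person character's HasKey1 when NeedKey is set.
; A FlipFlop plays or reverses the Rotate timeline, scaling door yaw by RotationZ.
; Locked and off-limits cases create a prompt widget with flavour text for that room.
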(event EventBeginPlay
  ;[1 1 1] Casting to First Person
  (bind _asfirst_person_character (Utilities|Casting|CastToFirstPersonCharacter (Game|GetPlayerCharacter 0)))
  (Variables|Default|SetPlayer%20Character _asfirst_person_character))

(event EventInteract
  (params (Interacter :type Actor%20Object%20Reference))
  ;[1 1 1] Checks For Key
  (if (Variables|Default|GetParentsBedroom?)
    (if (Variables|Default|GetNeedKey?)
      (if (Variables|/Game/FirstPersonBP/Blueprints/FirstPersonCharacter.FirstPersonCharacter_C|GetHasKey1? (Variables|Default|GetPlayer%20Character))
        (Utilities|FlowControl|FlipFlop :!label _label
          (:A
            (bind _rotateblend (Timeline|Rotate PlayFromStart)
              (:Update
                (Transformation|SetRelativeRotation (Variables|Default|GetDoor) (Math|Rotator|MakeRotator 0.0 0.0 (* _rotateblend (Variables|Default|GetRotation%20Z))) false false))))
          (:B
            (Timeline|Rotate ReverseFromEnd)))
        (else
          (bind _returnvalue (UserInterface|CreateWidget "/Game/Sven/LockAndKey/DoorLockedPrompt1.DoorLockedPrompt1_C"))
          (bind _output_get (Variables|Default|SetUI%20Door%20Prompt _returnvalue))
          (Variables|/Game/Sven/LockAndKey/DoorLockedPrompt1.DoorLockedPrompt1_C|SetDoor%20Prompt%20Body _output_get "Hmm. It's locked.")
          (UserInterface|Viewport|AddtoViewport _output_get 0)))
      (else
        (goto _label)))
    (elif (Variables|Default|GetMarthaBedroom)
      (bind _returnvalue_2 (UserInterface|CreateWidget "/Game/Sven/LockAndKey/DoorLockedPrompt1.DoorLockedPrompt1_C"))
      (bind _output_get_2 (Variables|Default|SetUI%20Door%20Prompt _returnvalue_2))
      (Variables|/Game/Sven/LockAndKey/DoorLockedPrompt1.DoorLockedPrompt1_C|SetDoor%20Prompt%20Body _output_get_2 "Grandma is sleeping right now. Better not bother her.")
      (UserInterface|Viewport|AddtoViewport _output_get_2 0)
      (else
        (bind _returnvalue_3 (UserInterface|CreateWidget "/Game/Sven/LockAndKey/DoorLockedPrompt1.DoorLockedPrompt1_C"))
        (bind _output_get_3 (Variables|Default|SetUI%20Door%20Prompt _returnvalue_3))
        (Variables|/Game/Sven/LockAndKey/DoorLockedPrompt1.DoorLockedPrompt1_C|SetDoor%20Prompt%20Body _output_get_3 "I'm not allowed in Marte's old bedroom.")
        (UserInterface|Viewport|AddtoViewport _output_get_3 0)))))

(fn ConstructionScript)